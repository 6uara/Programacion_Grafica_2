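; Actor that records a trail of player 0's movement as points on its spline component.
; On BeginPlay and every Tick, it compares the player location to the spline point queried at index -1.
; Beyond MinDistance, it appends the player location in world space and removes the oldest point once the count exceeds MaxPoints, keeping a rolling trail.
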(event EventBeginPlay
  (bind _spline (Variables|Default|GetSpline))
  ;[0.15 0.15 0.15 0.5] Get Distance to Player
  (Variables|Default|SetPLocation (Transformation|GetActorLocation (Game|GetPlayerCharacter 0)))
  (if (> (Math|Vector|Distance(Vector) (Spline|GetLocationatSplinePoint (Variables|Default|GetSpline) -1 "World") (Variables|Default|GetPLocation)) (Variables|Default|GetMinDistance))
    (Spline|AddSplinePoint (Variables|Default|GetSpline) (Variables|Default|GetPLocation) "World" true)
    (if (> (Spline|GetNumberOfSplinePoints _spline) (Variables|Default|GetMaxPoints))
      (Spline|RemoveSplinePoint _spline 0 true))))

(event Collision|EventActorBeginOverlap
  (params (OtherActor :type Actor%20Object%20Reference)))

(event EventTick
  (params (DeltaSeconds :type Float%20%28single-precision%29))
  (bind _spline (Variables|Default|GetSpline))
  (Variables|Default|SetPLocation (Transformation|GetActorLocation (Game|GetPlayerCharacter 0)))
  (if (> (Math|Vector|Distance(Vector) (Spline|GetLocationatSplinePoint (Variables|Default|GetSpline) -1 "World") (Variables|Default|GetPLocation)) (Variables|Default|GetMinDistance))
    (Spline|AddSplinePoint (Variables|Default|GetSpline) (Variables|Default|GetPLocation) "World" true)
    (if (> (Spline|GetNumberOfSplinePoints _spline) (Variables|Default|GetMaxPoints))
      (Spline|RemoveSplinePoint _spline 0 true))))

(fn ConstructionScript)